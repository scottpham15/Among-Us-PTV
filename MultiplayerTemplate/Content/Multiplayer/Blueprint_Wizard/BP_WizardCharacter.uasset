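; Player character for a multiplayer social-deduction game with kills, body reports, meetings and vents.
; BeginPlay sends the local player name to the server, registers minimap icons on clients, and binds body-proximity and end-game events to the controller's report button and GM_Master.
; RepNotifies update the overhead name, start meetings on authority and hide vented players with Ghost collision.
; Server events grant or clear the GAS kill ability, which debug key K activates.
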(event Custom|Server%20Set%20Player%20Name
  (params (PlayerName :type Text))
  (Variables|Default|SetPlayerName PlayerName))

(event Custom|Server%20Give%20Ability
  (bind _returnvalue (GameplayAbilities|GiveAbility (Variables|Default|GetAbilitySystemComponent) "/Game/Multiplayer/Blueprint_Wizard/GAS/GA_KillCrewMate.GA_KillCrewMate_C" 0 -1))
  (Variables|Default|SetNewVar _returnvalue))

(event Custom|Announcement
  (params (DeadBodyDes :type Dead%20Body%20Object%20Reference))
  (Variables|Default|SetDead%20Body%20Des DeadBodyDes)
  (bind _asbp_wizard_controller (Utilities|Casting|CastToBP_WizardController (Pawn|GetController)))
  (Default|TurnonReportButton _asbp_wizard_controller))

(event Custom|Announcement2
  (bind _asbp_wizard_controller (Utilities|Casting|CastToBP_WizardController (Pawn|GetController)))
  (Default|TurnOffReportButton _asbp_wizard_controller))

(event Custom|Check%20End%20Game
  (Utilities|FlowControl|Delay 3.0)
  (bind _asgm_master (Utilities|Casting|CastToGM_Master (Game|GetGameMode)))
  (Default|CheckWin/Lose _asgm_master))

(event Custom|Server%20Clear%20Ability
  (GameplayAbilities|ClearAbility (Variables|Default|GetAbilitySystemComponent) (Variables|Default|GetNewVar)))

(event EventBeginPlay
  (bind _returnvalue (Class|GameplayStatics|GetPlayerControllerfromID))
  (bind _self self)
  (bind _returnvalue_2 (Subsystems|GetMinimapSubsystem _returnvalue))
  (Utilities|FlowControl|Sequence
    (:then_0
      (CallFunction|SetUpLocal)
      (Networking|SwitchHasAuthority
        (:Remote
          (if (Pawn|IsLocallyControlled)
            (Class|MinimapSubsystem|RegisterMainCharacterEntry _returnvalue_2 _self false "/Game/Multiplayer/Widgets/MainMenu/Characters/Manny_Red.Manny_Red")
            (else
              (Class|MinimapSubsystem|RegisterEntry _returnvalue_2 _self false "/Game/Multiplayer/Widgets/MainMenu/Characters/Manny.Manny"))))))
    (:then_1
      (EventDispatchers|BindEventtoFoundDeadBody (delegate Custom|Announcement)))
    (:then_2
      (EventDispatchers|BindEventtoAwayfromDeadBody (delegate Custom|Announcement2)))
    (:then_3
      (EventDispatchers|BindEventtoCheckEndGame (delegate Custom|Check%20End%20Game)))))

(event Input|KeyboardEvents|DebugKeyK
  (params (Key :type Key%20Structure :default "None") (ActionValue :type Input%20Action%20Value%20Structure))
  (:Pressed
    (Abilities|TryActivateAbilitybyClass (Variables|Default|GetAbilitySystemComponent) "/Game/Multiplayer/Blueprint_Wizard/GAS/GA_KillCrewMate.GA_KillCrewMate_C" true)))

(fn ConstructionScript)

(fn ChangeColorName
  (bind _aswb_name_on_head (Utilities|Casting|CastToWB_NameOnHead (UserInterface|GetWidget (Variables|Default|GetNameOnHead_0))))
  (Appearance|SetColorandOpacity (Variables|/Game/Demo/ThirdPerson/Blueprints/WB_NameOnHead.WB_NameOnHead_C|GetNameText _aswb_name_on_head) (Utilities|Struct|MakeSlateColor "(R=0.651042,G=0.000000,B=0.020048,A=1.000000)") :!class /Script/UMG.TextBlock))

(fn OnRepPlayerName
  (bind _nameonhead_0 (Variables|Default|GetNameOnHead_0))
  (bind _returnvalue (UserInterface|GetWidget _nameonhead_0))
  (Utilities|IsValid _returnvalue
    (:Is%20Valid
      (bind _aswb_name_on_head (Utilities|Casting|CastToWB_NameOnHead _returnvalue))
      (Default|SetName _aswb_name_on_head (Variables|Default|GetPlayerName))
      (Development|SetHiddeninGame (Variables|Default|GetNameOnHead_0) false false))
    (:Is%20Not%20Valid
      (Utilities|Time|SetTimerbyFunctionName 0 "OnRep_PlayerName" 0.1))))

(fn SetUpLocal
  (if (Pawn|IsLocallyControlled)
    (bind _asbp_game_instance (Utilities|Casting|CastToBP_GameInstance (Game|GetGameInstance)))
    (CallFunction|ServerSetPlayerName (Variables|/Game/Multiplayer/BP_GameInstance.BP_GameInstance_C|GetPlayerName _asbp_game_instance))))

(fn OnRepClickReportedButton
  (Networking|SwitchHasAuthority
    (:Authority
      (bind _asgm_master (Utilities|Casting|CastToGM_Master (Game|GetGameMode)))
      (bind _asbp_wizard_controller (Utilities|Casting|CastToBP_WizardController (Pawn|GetController)))
      (Default|Meeting _asgm_master (Variables|/Game/Multiplayer/Blueprint_Wizard/BP_WizardController.BP_WizardController_C|GetEmergencyOrDeadbody _asbp_wizard_controller)))))

(fn OnRepHiddenonJumptoVent
  (Collision|SetCollisionProfileName (Variables|Default|GetCapsuleComponent) (select (Variables|Default|GetHiddenOnJumpToVent) "Ghost" "Pawn") false :!class /Script/Engine.PrimitiveComponent)
  (Rendering|SetActorHiddenInGame (Variables|Default|GetHiddenOnJumpToVent)))