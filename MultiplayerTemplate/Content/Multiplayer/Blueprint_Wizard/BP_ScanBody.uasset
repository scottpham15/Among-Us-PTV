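; Body-scan task station for non-imposter wizards in a multiplayer imposter game, shown on their minimap as a static icon on remote clients.
; A server-side box overlap starts the scan through the player's controller, and Tick sweeps the actor up and back down.
; A completed sweep ends the scan and updates game mode progress through the controller.
; Leaving the box stops the sweep, resets it to a hard-coded position and cancels the scan.
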(event `self.ReceiveBeginPlay`
  (bind _returnvalue (`GameplayStatics.GetPlayerControllerFromID` 0))
  (`/Engine/EditorBlueprintResources/ActorMacros.Switch Has Authority`
    (:`Remote`
      (bind _asbp_wizard_character (cast `/Game/Multiplayer/Blueprint_Wizard/BP_WizardCharacter` (`Controller.K2_GetPawn` _returnvalue)))
      (if (not (`/Game/Multiplayer/Blueprint_Wizard/BP_WizardCharacter.bImposter` _asbp_wizard_character))
        (`MinimapSubsystem.RegisterEntry` (pcsubsystem `MinimapSubsystem` _returnvalue) self false "/Game/Multiplayer/Widgets/Texture/body-1.body-1")))))

(event `self.ReceiveTick`
  (params (DeltaSeconds :type "Float (single-precision)"))
  (bind (_returnvalue_x _returnvalue_y _returnvalue_z) (`KismetMathLibrary.BreakVector` (`self.K2_GetActorLocation`)))
  (bind (_returnvalue_x_2 _returnvalue_y_2 _returnvalue_z_2) (`KismetMathLibrary.BreakVector` (`self.K2_GetActorLocation`)))
  (bind _as_bp_wizard_controller (`self.As BP Wizard Controller`))
  (if (`self.Start`)
    (`self.K2_SetActorLocation` (`KismetMathLibrary.MakeVector` _returnvalue_x_2 _returnvalue_y_2 (+ _returnvalue_z_2 (`self.UpDown`))))
    (if (> _returnvalue_z 720.0)
      (set `self.UpDown` -0.7)
      (elif (< _returnvalue_z 590.0)
        (set `self.UpDown` 0.0)
        (set `self.Start` false)
        (`/Game/Multiplayer/Blueprint_Wizard/BP_WizardController.Server Cancel Scan Body` _as_bp_wizard_controller)
        (`/Game/Multiplayer/Blueprint_Wizard/BP_WizardController.Server Set Percent Gamemode` _as_bp_wizard_controller)))))

(event `self.Box.OnComponentBeginOverlap`
  (params (OverlappedComponent :type "PrimitiveComponent Object Reference") (OtherActor :type "Actor Object Reference") (OtherComp :type "PrimitiveComponent Object Reference") (OtherBodyIndex :type Integer) (bFromSweep :type Boolean) (SweepResult :type "HitResult Structure (by ref)"))
  (`/Engine/EditorBlueprintResources/ActorMacros.Switch Has Authority`
    (:`Authority`
      (bind _asbp_wizard_character (cast `/Game/Multiplayer/Blueprint_Wizard/BP_WizardCharacter` OtherActor))
      (bind _asbp_wizard_controller (cast `/Game/Multiplayer/Blueprint_Wizard/BP_WizardController` (`Pawn.GetController` _asbp_wizard_character)))
      (if (not (`/Game/Multiplayer/Blueprint_Wizard/BP_WizardCharacter.bImposter` _asbp_wizard_character))
        (set `self.As BP Wizard Controller` _asbp_wizard_controller)
        (set `self.Start` true)
        (`/Game/Multiplayer/Blueprint_Wizard/BP_WizardController.Server Scan Body` (`self.As BP Wizard Controller`))))))

(event `self.Box.OnComponentEndOverlap`
  (params (OverlappedComponent :type "PrimitiveComponent Object Reference") (OtherActor :type "Actor Object Reference") (OtherComp :type "PrimitiveComponent Object Reference") (OtherBodyIndex :type Integer))
  (`/Engine/EditorBlueprintResources/ActorMacros.Switch Has Authority`
    (:`Authority`
      (set `self.Start` false)
      (`self.K2_SetActorLocation` (1250.0 -150.0 590.0))
      (set `self.UpDown` 0.7)
      (bind _asbp_wizard_character (cast `/Game/Multiplayer/Blueprint_Wizard/BP_WizardCharacter` OtherActor))
      (if (not (`/Game/Multiplayer/Blueprint_Wizard/BP_WizardCharacter.bImposter` _asbp_wizard_character))
        (bind _asbp_wizard_controller (cast `/Game/Multiplayer/Blueprint_Wizard/BP_WizardController` (`Pawn.GetController` _asbp_wizard_character)))
        (`/Game/Multiplayer/Blueprint_Wizard/BP_WizardController.Server Cancel Scan Body` _asbp_wizard_controller)))))

(fn `UserConstructionScript`)