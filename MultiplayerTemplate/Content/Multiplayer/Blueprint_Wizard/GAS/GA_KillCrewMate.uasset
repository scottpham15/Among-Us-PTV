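; Gameplay ability that kills a nearby crewmate wizard, teleporting the attacker onto the victim.
; A debug-drawn sphere overlap at a fixed height finds other wizards; imposters and ghosts trigger CancelAbility.
; The first valid target receives GE_ReduceHealth, then the loop breaks and a 2D sound and attack montage play.
; CommitAbility runs only after the montage, if the hit flag NewVar is set, before the ability ends.
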(event `self.K2_ActivateAbility`
  (bind _returnvalue (`self.GetAvatarActorFromActorInfo`))
  (bind (_returnvalue_x _returnvalue_y) (`KismetMathLibrary.BreakVector` (`Actor.K2_GetActorLocation` _returnvalue)))
  (`KismetSystemLibrary.DrawDebugSphere` (`KismetMathLibrary.MakeVector` _returnvalue_x _returnvalue_y 550.0) 300.0 12 (struct :`R` 1.0 :`B` 0.376997 :`A` 1.0) 1.0)
  (bind (_outactors _returnvalue_2) (`KismetSystemLibrary.SphereOverlapActors` (`KismetMathLibrary.MakeVector` _returnvalue_x _returnvalue_y 550.0) 300.0 (`|MakeArray` "ObjectTypeQuery3" :!type "EObjectTypeQuery Enum") "/Game/Multiplayer/Blueprint_Wizard/BP_WizardCharacter.BP_WizardCharacter_C" (`|MakeArray` _returnvalue)))
  (for _array_element _outactors
    (if _returnvalue_2
      (bind _asbp_wizard_character (cast `/Game/Multiplayer/Blueprint_Wizard/BP_WizardCharacter` _array_element))
      (if (`/Game/Multiplayer/Blueprint_Wizard/BP_WizardCharacter.bImposter` _asbp_wizard_character)
        _
        (elif (`MyCharacter.IsGhost` _asbp_wizard_character)
          _
          (else
            (`AbilitySystemComponent.BP_ApplyGameplayEffectSpecToSelf` (`AbilitySystemBlueprintLibrary.GetAbilitySystemComponent` _array_element) (`self.MakeOutgoingGameplayEffectSpec` "/Game/Multiplayer/Blueprint_Wizard/GAS/GE_ReduceHealth.GE_ReduceHealth_C"))
            (`Actor.K2_SetActorLocation` (`self.GetAvatarActorFromActorInfo`) (`Actor.K2_GetActorLocation` _asbp_wizard_character) false true)
            (set `self.NewVar` true)
            (break)))))
    (`self.K2_CancelAbility`))
  (`GameplayStatics.PlaySound2D` "/Game/Multiplayer/Widgets/Texture/stationary-kill_gDwMUvN.stationary-kill_gDwMUvN" 1.0 1.0 0.0 null null)
  (`AbilityTask_PlayMontageAndWait.CreatePlayMontageAndWaitProxy` "None" "/Game/BattleWizardPolyart/AM_AttackWizard.AM_AttackWizard"
    (:`OnCompleted`
      _)
    (:`OnBlendOut`
      _)
    (:`OnInterrupted`
      _)
    (:`OnCancelled`
      _))
  (if (`self.NewVar`)
    (`self.K2_CommitAbility`))
  (`self.K2_EndAbility`))