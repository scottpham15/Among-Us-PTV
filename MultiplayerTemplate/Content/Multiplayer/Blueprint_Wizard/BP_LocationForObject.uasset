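; BP_LocationForObject is a drop-off slot where a wizard player deposits a transported object.
; When a wizard overlaps its Box while the slot is Empty, the server takes the transport object referenced by that player's controller.
; It attaches the object to itself, hands it a back-reference through BPLocation, clears the controller's reference and marks the slot occupied.
; Nothing in this Blueprint resets Empty.
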(event `self.Box.OnComponentBeginOverlap`
  (params (OverlappedComponent :type "PrimitiveComponent Object Reference") (OtherActor :type "Actor Object Reference") (OtherComp :type "PrimitiveComponent Object Reference") (OtherBodyIndex :type Integer) (bFromSweep :type Boolean) (SweepResult :type "HitResult Structure (by ref)"))
  (`/Engine/EditorBlueprintResources/ActorMacros.Switch Has Authority`
    (:`Authority`
      (if (`self.Empty`)
        (bind _asbp_wizard_character (cast `/Game/Multiplayer/Blueprint_Wizard/BP_WizardCharacter` OtherActor))
        (bind _asbp_wizard_controller (cast `/Game/Multiplayer/Blueprint_Wizard/BP_WizardController` (`Pawn.GetController` _asbp_wizard_character)))
        (bind _as_bp_object_transport (`/Game/Multiplayer/Blueprint_Wizard/BP_WizardController.As BP Object Transport` _asbp_wizard_controller))
        (`/Engine/EditorBlueprintResources/StandardMacros.IsValid` _as_bp_object_transport
          (:`Is Valid`
            (set `/Game/Multiplayer/Blueprint_Wizard/BP_ObjectTransport.BP Location` self _as_bp_object_transport)
            (`self.K2_AttachToActor` _as_bp_object_transport self "None" "KeepRelative" "KeepRelative" "KeepWorld" true)
            (set `/Game/Multiplayer/Blueprint_Wizard/BP_WizardController.As BP Object Transport` null _asbp_wizard_controller)
            (set `self.Empty` false)))))))

(fn `UserConstructionScript`)