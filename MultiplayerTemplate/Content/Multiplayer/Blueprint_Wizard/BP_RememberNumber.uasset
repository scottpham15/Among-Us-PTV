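; BP_RememberNumber is a multiplayer interactable actor tied to the wizard player who is its Instigator.
; On remote instances, it registers a moving Number icon on the minimap only if the local pawn is that Instigator.
; On the authority, its Sphere overlap sets the instigating wizard controller's use type and turns on the Use button.
; Leaving the sphere turns the button off, and other characters are ignored.
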(event `self.ReceiveBeginPlay`
  (bind _returnvalue (`GameplayStatics.GetPlayerControllerFromID` 0))
  (`/Engine/EditorBlueprintResources/ActorMacros.Switch Has Authority`
    (:`Remote`
      (if (== (`Controller.K2_GetPawn` _returnvalue) (`self.Instigator`))
        (`MinimapSubsystem.RegisterEntry` (pcsubsystem `MinimapSubsystem` _returnvalue) self false "/Game/Multiplayer/Widgets/Texture/number.number")))))

(event `self.Sphere.OnComponentBeginOverlap`
  (params (OverlappedComponent :type "PrimitiveComponent Object Reference") (OtherActor :type "Actor Object Reference") (OtherComp :type "PrimitiveComponent Object Reference") (OtherBodyIndex :type Integer) (bFromSweep :type Boolean) (SweepResult :type "HitResult Structure (by ref)"))
  (`/Engine/EditorBlueprintResources/ActorMacros.Switch Has Authority`
    (:`Authority`
      (bind _asbp_wizard_character (cast `/Game/Multiplayer/Blueprint_Wizard/BP_WizardCharacter` OtherActor))
      (if (== _asbp_wizard_character (`self.GetInstigator`))
        (bind _asbp_wizard_controller (cast `/Game/Multiplayer/Blueprint_Wizard/BP_WizardController` (`Pawn.GetController` _asbp_wizard_character)))
        (set `/Game/Multiplayer/Blueprint_Wizard/BP_WizardController.WhatUse` 2 _asbp_wizard_controller)
        (`/Game/Multiplayer/Blueprint_Wizard/BP_WizardController.Turn On Use Button` _asbp_wizard_controller)))))

(event `self.Sphere.OnComponentEndOverlap`
  (params (OverlappedComponent :type "PrimitiveComponent Object Reference") (OtherActor :type "Actor Object Reference") (OtherComp :type "PrimitiveComponent Object Reference") (OtherBodyIndex :type Integer))
  (`/Engine/EditorBlueprintResources/ActorMacros.Switch Has Authority`
    (:`Authority`
      (bind _asbp_wizard_character (cast `/Game/Multiplayer/Blueprint_Wizard/BP_WizardCharacter` OtherActor))
      (if (== _asbp_wizard_character (`self.GetInstigator`))
        (bind _asbp_wizard_controller (cast `/Game/Multiplayer/Blueprint_Wizard/BP_WizardController` (`Pawn.GetController` _asbp_wizard_character)))
        (`/Game/Multiplayer/Blueprint_Wizard/BP_WizardController.Turn Off Use Button` _asbp_wizard_controller)))))

(fn `UserConstructionScript`)